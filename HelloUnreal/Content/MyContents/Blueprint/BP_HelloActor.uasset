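; Actor that moves its Sphere component around a roughly square loop using relative offsets on Tick.
; Each frame advances along X or Y by DeltaSeconds times Speed, accumulating distance until it passes 1000 units and switches axis.
; A turn counter flips direction after every two legs, so the forward pair is retraced in reverse signs to close the loop.
; Disconnected experiments with back-and-forth movement, loops, printing and transforms remain and never run.
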(event `self.ReceiveBeginPlay`)

(event `self.ReceiveTick`
  (params (DeltaSeconds :type "Float (single-precision)"))
  (bind _returnvalue (* DeltaSeconds (`self.Speed`)))
  (bind _returnvalue_2 (* DeltaSeconds (`self.Speed`)))
  (bind _returnvalue_3 (* DeltaSeconds (`self.Speed`)))
  (bind _returnvalue_4 (* DeltaSeconds (`self.Speed`)))
  (if (`self.IsTurn?`)
    ;[1 1 1] 정방향
    (if (`self.IsXMove?`)
      ;;[1 1 1] X방향
      (bind _output_get (set `self.X_Distance` (+ (`self.X_Distance`) _returnvalue_4)))
      (`SceneComponent.K2_AddRelativeLocation` (`self.Sphere`) (`KismetMathLibrary.MakeVector` _returnvalue_4) false false)
      (if (> _output_get 1000.0)
        (set `self.X_Distance` 0.0)
        (set `self.IsXMove?` false)
        (bind _output_get_2 (set `self.TurnCount` (+ (`self.TurnCount`) 1.0) :!label _label))
        (if (>= _output_get_2 2.0)
          (set `self.TurnCount` 0.0)
          (set `self.IsTurn?` false)))
      (else
        ;;[1 1 1] Y방향
        (bind _output_get_3 (set `self.Y_Distance` (+ (`self.Y_Distance`) _returnvalue_3)))
        (`SceneComponent.K2_AddRelativeLocation` (`self.Sphere`) (`KismetMathLibrary.MakeVector` 0.0 _returnvalue_3) false false)
        (if (> _output_get_3 1000.0)
          (set `self.Y_Distance` 0.0)
          (set `self.IsXMove?` true)
          (goto _label))))
    (else
      ;[1 1 1] 역방향
      (if (`self.IsXMove?`)
        ;;[1 1 1] X방향
        (bind _output_get_4 (set `self.X_Distance` (+ (`self.X_Distance`) _returnvalue)))
        (`SceneComponent.K2_AddRelativeLocation` (`self.Sphere`) (`KismetMathLibrary.MakeVector` (* _returnvalue -1.0)) false false)
        (if (> _output_get_4 1000.0)
          (set `self.X_Distance` 0.0)
          (set `self.IsXMove?` false)
          (bind _output_get_5 (set `self.TurnCount` (+ (`self.TurnCount`) 1.0) :!label _label_2))
          (if (>= _output_get_5 2.0)
            (set `self.TurnCount` 0.0)
            (set `self.IsTurn?` true)))
        (else
          ;;[1 1 1] Y방향
          (bind _output_get_6 (set `self.Y_Distance` (+ (`self.Y_Distance`) _returnvalue_2)))
          (`SceneComponent.K2_AddRelativeLocation` (`self.Sphere`) (`KismetMathLibrary.MakeVector` 0.0 (* _returnvalue_2 -1.0)) false false)
          (if (> _output_get_6 1000.0)
            (set `self.Y_Distance` 0.0)
            (set `self.IsXMove?` true)
            (goto _label_2)))))))

(fn `UserConstructionScript`)